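; BP_TPSAIController is an AI controller for the TPS game that currently does nothing, as its Tick, Possess and MoveToRandomLocation events are empty.
; Its disconnected graphs hold movement experiments: seeking the player character or a target point, old trace-and-steer logic, and running BT_AIDefault.
; Another unwired chain picks random navigable locations and calls MoveToRandomLocation again when the lookup or move request fails.
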(event Custom|MoveToRandomLocation
  ;[1 0 0 0.5] to random target
)

(event EventPossess
  (params (PossessedPawn :type Pawn%20Object%20Reference)))

(event EventTick
  (params (DeltaSeconds :type Float%20%28single-precision%29)))

(fn ConstructionScript)