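; BP_BaseItem is a base item actor that can be picked up into an inventory through an Interact event.
; On BeginPlay it copies its quantity into the BPCItomInventory component, which also holds the item's data row.
; Interact passes that row name and quantity to the interacting actor's BAC_InventorySystem.
; A successful add destroys the item; otherwise the component keeps the remaining quantity.
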(event EventBeginPlay
  (Variables|/Game/TPS/Components/Inventory/BAC_ItemInventory.BAC_ItemInventory_C|SetQuanity (Variables|Default|GetBPC_ItomInventory) (Variables|Default|GetQuanity)))

(event Collision|EventActorBeginOverlap
  (params (OtherActor :type Actor%20Object%20Reference)))

(event EventTick
  (params (DeltaSeconds :type Float%20%28single-precision%29)))

(event EventInteract
  (params (Actor :type Actor%20Object%20Reference))
  (bind _returnvalue (Actor|GetComponentbyClass Actor "/Game/TPS/Components/Inventory/BAC_InventorySystem.BAC_InventorySystem_C"))
  (bind _bpc_itominventory (Variables|Default|GetBPC_ItomInventory))
  (Utilities|IsValid _returnvalue
    (:Is%20Valid
      (bind (_bissuccess _quanityremain) (Default|AddtoInventory _returnvalue (.rowname (Variables|/Game/TPS/Components/Inventory/BAC_ItemInventory.BAC_ItemInventory_C|GetItemData _bpc_itominventory)) (Variables|/Game/TPS/Components/Inventory/BAC_ItemInventory.BAC_ItemInventory_C|GetQuanity _bpc_itominventory)))
      (if _bissuccess
        (Actor|DestroyActor)
        (else
          (Variables|/Game/TPS/Components/Inventory/BAC_ItemInventory.BAC_ItemInventory_C|SetQuanity (Variables|Default|GetBPC_ItomInventory) _quanityremain))))))

(fn ConstructionScript)