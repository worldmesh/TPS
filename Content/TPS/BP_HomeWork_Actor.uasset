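; Homework actor Blueprint that exercises health and line-trace functions, with calls to parent implementations.
; On BeginPlay it sets Health, reads it back through GetHealth and prints it on screen, while NotifyActor prints a given actor's name.
; TraceForPhysicsBody calls the parent, then runs a debug-drawn Visibility trace to GetTraceLocation, returning the hit actor, component and blocking result.
; A looping timer is disconnected, and a local forward-vector endpoint helper is unused.
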(event Custom|TraceOfObject
  ;[0 1 0 0.5] HW 6 Trace
)

(event EventBeginPlay
  (|CallParentFunction)
  (Utilities|FlowControl|Sequence
    (:then_0
      ;[0 1 0 0.5] HW 5 Print Health
      (Variables|Default|SetHealth 1e+02)
      (bind _returnvalue (Class|HomeWorkActor|GetHealth))
      (Development|PrintString (Utilities|String|ToString(Float) _returnvalue) true true "(R=1.000000,G=0.000000,B=0.000000,A=1.000000)" 5.0))))

(event Collision|EventActorBeginOverlap
  (params (OtherActor :type Actor%20Object%20Reference)))

(event EventTick
  (params (DeltaSeconds :type Float%20%28single-precision%29)))

(event EventNotifyActor
  (params (Actor :type Actor%20Object%20Reference))
  ;[0 1 0 0.5] HW 6 Trace
  (Development|PrintString (Utilities|GetDisplayName Actor)))

(fn ConstructionScript)

(fn GetTraceLocation0
  (return (+ (Transformation|GetActorLocation) (* (Math|Vector|GetForwardVector (Transformation|GetActorRotation)) (Variables|Default|GetMaxTraceDistance_0)))))

(fn TraceforPhysicsBody
  (|CallParentFunction)
  (bind _outhit (Collision|LineTraceByChannel (Transformation|GetActorLocation) (Class|HomeWorkActor|GetTraceLocation) "TraceTypeQuery1" false 0 "ForOneFrame"))
  (return (.HitActor (Collision|BreakHitResult _outhit)) (.HitComponent (Collision|BreakHitResult _outhit)) (.bBlockingHit (Collision|BreakHitResult _outhit))))